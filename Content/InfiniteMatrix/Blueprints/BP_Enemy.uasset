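; BP_Enemy is an enemy actor that reacts to overlaps with the player or a bullet.
; Touching BP_Player cuts the player's health by a fixed amount through UpdateHealth and destroys the enemy.
; Touching BP_Bullet adds a point to the score of player pawn 0 through UpdateScore and destroys the enemy.
; All logic runs in ActorBeginOverlap using casts, with no movement or Tick logic in this graph.
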(event `self.ReceiveActorBeginOverlap`
  (params (OtherActor :type "Actor Object Reference"))
  (bind _asbp_player (cast `/Game/InfiniteMatrix/Blueprints/BP_Player` OtherActor)
    (:`then`
      (`/Game/InfiniteMatrix/Blueprints/BP_Player.UpdateHealth` _asbp_player (- (`/Game/InfiniteMatrix/Blueprints/BP_Player.Health` _asbp_player) 30.0))
      (`self.K2_DestroyActor`))
    (:`CastFailed`
      (cast `/Game/InfiniteMatrix/Blueprints/BP_Bullet` OtherActor)
      (bind _asbp_player_2 (cast `/Game/InfiniteMatrix/Blueprints/BP_Player` (`GameplayStatics.GetPlayerPawn` 0)))
      (`/Game/InfiniteMatrix/Blueprints/BP_Player.UpdateScore` _asbp_player_2 (+ (`/Game/InfiniteMatrix/Blueprints/BP_Player.Score` _asbp_player_2) 1))
      (`self.K2_DestroyActor`))))

(fn `UserConstructionScript`)