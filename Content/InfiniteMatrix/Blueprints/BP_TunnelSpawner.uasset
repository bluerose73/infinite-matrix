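; BP_TunnelSpawner builds a chain of BP_Tunnel segments, clearing existing ones at BeginPlay and seeding a few from the player's location.
; Each new segment attaches at the newest tunnel's SpawnPoint, receives a spawner reference and randomizes its wall.
; Low player health gives new segments a danger material.
; Each spawn may also randomly place a short-lived health pack or, more often, an enemy ahead with random offset.
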(event `self.ReceiveBeginPlay`
  (`self.SpawnInitialTunnels`))

(fn `SpawnInitialTunnels`
  (`|ExecutionSequence`
    (:`then_0`
      (bind _outactors (`GameplayStatics.GetAllActorsOfClass` "/Game/InfiniteMatrix/Blueprints/BP_Tunnel.BP_Tunnel_C"))
      (for _array_element _outactors
        (`self.K2_DestroyActor` _array_element)))
    (:`then_1`
      (for _ (range 3)
        (`/Engine/EditorBlueprintResources/StandardMacros.IsValid` (`self.NewestTunnel`)
          (:`Is Valid`
            (`self.SpawnTunnelFromSpawnPoint`))
          (:`Is Not Valid`
            (`self.SpawnTunnel` (`self.K2_GetActorLocation` (`GameplayStatics.GetPlayerPawn` 0)))))))))

(fn `SpawnTunnel`
  (params (SpawnLocation :type "Vector Structure"))
  (bind _returnvalue (`KismetMathLibrary.RandomIntegerInRange` 0 9))
  (bind _returnvalue_2 (+ SpawnLocation (`KismetMathLibrary.MakeVector` 2000.0 (`KismetMathLibrary.RandomFloatInRange` -200.0 200.0) (`KismetMathLibrary.RandomFloatInRange` -200.0 200.0))))
  (`|ExecutionSequence`
    (:`then_0`
      (bind _returnvalue_3 (`|SpawnActorFromClass` "/Game/InfiniteMatrix/Blueprints/BP_Tunnel.BP_Tunnel_C" (`KismetMathLibrary.MakeTransform` SpawnLocation) "Undefined" "MultiplyWithRoot" null null))
      (bind _output_get (set `self.NewestTunnel` _returnvalue_3))
      (set `/Game/InfiniteMatrix/Blueprints/BP_Tunnel.TunnelSpawner` self _output_get)
      (`/Game/InfiniteMatrix/Blueprints/BP_Tunnel.RandomizeWall` _output_get)
      (bind _asbp_player (cast `/Game/InfiniteMatrix/Blueprints/BP_Player` (`GameplayStatics.GetPlayerPawn` 0)))
      (if (< (`/Game/InfiniteMatrix/Blueprints/BP_Player.Health` _asbp_player) 30.0)
        (`PrimitiveComponent.SetMaterial` (`StaticMeshActor.StaticMeshComponent` _returnvalue_3) 0 "/Game/InfiniteMatrix/Materials/MI_TunnelDanger.MI_TunnelDanger")))
    (:`then_1`
      (if (>= _returnvalue 8)
        (bind _returnvalue_4 (`|SpawnActorFromClass` "/Game/InfiniteMatrix/Blueprints/BP_HealthPack.BP_HealthPack_C" (`KismetMathLibrary.MakeTransform` _returnvalue_2) "Undefined" "MultiplyWithRoot" null null))
        (`self.SetLifeSpan` _returnvalue_4 20.0)
        (elif (>= _returnvalue 2)
          (bind _returnvalue_5 (`|SpawnActorFromClass` "/Game/InfiniteMatrix/Blueprints/BP_Enemy.BP_Enemy_C" (`KismetMathLibrary.MakeTransform` _returnvalue_2) "Undefined" "MultiplyWithRoot" null null))
          (`self.SetLifeSpan` _returnvalue_5 20.0))))))

(fn `SpawnTunnelFromSpawnPoint`
  (`self.SpawnTunnel` (`SceneComponent.K2_GetComponentLocation` (`/Game/InfiniteMatrix/Blueprints/BP_Tunnel.SpawnPoint` (`self.NewestTunnel`)))))

(fn `UserConstructionScript`)